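; Test dialogue component that scripts a branching conversation between a test NPC and Charlie, overriding the parent Dialogue function.
; Chained AddDialogue calls supply lines, reply options, montages and some audio, branching on the selected option.
; Finishing the longest branch sets DialogueTreeIndex to 1, which switches later talks to a randomly chosen brush-off line.
; Every ending closes the conversation, and all others also clear dialogue progress.
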(fn `Dialogue`
  (`parent.Dialogue`)
  (switch `int` (`self.DialogueTreeIndex`)
    (:`0`
      (bind (_state _optionindex) (`self.AddDialogue` "Test" "Hi, Charlie! I'm a test NPC" (`|MakeArray` "Hi, Ms Frost!" "Who are you again?" :!type "Text") "/Game/Dialogue/Audio/1.1" "/Game/Characters/Animations/Rebecca_Manager/Having_A_Meeting__Female_mixamo_com_Montage.Having_A_Meeting__Female_mixamo_com_Montage"))
      (switch `/Game/Dialogue/Enum_DialogueState` _state
        (:`NewEnumerator0`
          (switch `int` _optionindex
            (:`0`
              (bind (_state_2 _optionindex_2) (`self.AddDialogue` "Test" "Charlie, Up for some trouble?" (`|MakeArray` "Yep, as always!" "Nope." :!type "Text") "/Game/Dialogue/Audio/2.2" "/Game/Characters/Animations/Rebecca_Manager/Having_A_Meeting__Female_mixamo_com_Montage.Having_A_Meeting__Female_mixamo_com_Montage"))
              (switch `/Game/Dialogue/Enum_DialogueState` _state_2
                (:`NewEnumerator0`
                  (switch `int` _optionindex_2
                    (:`0`
                      (bind (_state_3 _optionindex_3) (`self.AddDialogue` "Test" "Charlie, these boys are not good! You are going to end up like my husband Richard in Texas prison, my love." (`|MakeArray` "(keep listening)" :!type "Text") null "/Game/Characters/Animations/Rebecca_Manager/Having_A_Meeting__Female_mixamo_com_Montage.Having_A_Meeting__Female_mixamo_com_Montage"))
                      (switch `/Game/Dialogue/Enum_DialogueState` _state_3
                        (:`NewEnumerator0`
                          (switch `int` _optionindex_3
                            (:`0`
                              (bind _state_4 (`self.AddDialogue` "Test" "Oh, he was just like you, but better, strong, blond with brown eyes, He would drink beer non stop, omg I love him so much!" (`|MakeArray` "That's lovely, but I really have to go." :!type "Text") null "/Game/Characters/Animations/Rebecca_Manager/Having_A_Meeting__Female_mixamo_com_Montage.Having_A_Meeting__Female_mixamo_com_Montage"))
                              (switch `/Game/Dialogue/Enum_DialogueState` _state_4
                                (:`NewEnumerator0`
                                  (`self.SetDialogueTreeIndex` 1)
                                  (`self.CloseConversation`))))))))
                    (:`1`
                      (bind _state_5 (`self.AddDialogue` "Test" "Good! Say hi from me to your mom!" (`|MakeArray` "I will!" :!type "Text") null "/Game/Characters/Animations/Rebecca_Manager/Having_A_Meeting__Female_mixamo_com_Montage.Having_A_Meeting__Female_mixamo_com_Montage"))
                      (switch `/Game/Dialogue/Enum_DialogueState` _state_5
                        (:`NewEnumerator0`
                          (`self.ClearDialogueProgress`)
                          (`self.CloseConversation`))))))))
            (:`1`
              (bind _state_6 (`self.AddDialogue` "Test" "Well, don't be mean now! I'm going to tell your mom!" (`|MakeArray` "Sorry, but I honestly have no idea who you are." :!type "Text")))
              (switch `/Game/Dialogue/Enum_DialogueState` _state_6
                (:`NewEnumerator0`
                  (`self.ClearDialogueProgress`)
                  (`self.CloseConversation`))))))))
    (:`1`
      (bind _state_7 (`self.AddDialogue` "Test" (select `int` (`KismetMathLibrary.RandomIntegerInRange` 0 1) :`0` "Well, walk away! I'm a busy women I have no time for chat." :`1` "Boy, you're getting on my nervs" :!type "Text") (`|MakeArray` "Okay, miss thing!" :!type "Text") null "/Game/Characters/Animations/Rebecca_Manager/Having_A_Meeting__Female_mixamo_com_Montage.Having_A_Meeting__Female_mixamo_com_Montage"))
      (switch `/Game/Dialogue/Enum_DialogueState` _state_7
        (:`NewEnumerator0`
          (`self.ClearDialogueProgress`)
          (`self.CloseConversation`))))))