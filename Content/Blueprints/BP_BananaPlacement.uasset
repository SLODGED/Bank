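; BP_BananaPlacement is a puzzle spot where a dropped banana triggers Bob's fall cutscene.
; Overlapping BananaArea freezes the banana and blocks pickup; the cutscene starts once both that and SetReady have happened, in either order.
; It destroys bananas and Bob, hides and immobilizes the player, then plays a Level Sequence.
; On finish it restores the player, reveals the fallen Bob, readies chandeliers and destroys Chad.
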(event `self.ReceiveBeginPlay`
  (bind _bobfallen (`self.BobFallen`))
  (`SceneComponent.SetVisibility` _bobfallen false true)
  (`PrimitiveComponent.SetCollisionEnabled` _bobfallen "NoCollision"))

(event `self.BananaArea.OnComponentBeginOverlap`
  (params (OverlappedComponent :type "PrimitiveComponent Object Reference") (OtherActor :type "Actor Object Reference") (OtherComp :type "PrimitiveComponent Object Reference") (OtherBodyIndex :type Integer) (bFromSweep :type Boolean) (SweepResult :type "HitResult Structure (by ref)"))
  (bind _outactors (`GameplayStatics.GetAllActorsOfClass` "/Game/Blueprints/BP_Banana.BP_Banana_C"))
  (for _array_element _outactors
    (if (== OtherActor _array_element)
      (set `self.IsBananaInArea?` true)
      (`KismetSystemLibrary.PrintString` "BananaIsInArea")
      (`PrimitiveComponent.SetSimulatePhysics` (`/Game/Blueprints/BP_Banana.Banana` _array_element) false)
      (set `/Game/Blueprints/BP_Banana.CanPickup` false _array_element)
      (set `/Game/Blueprints/BP_Banana.IsBananaInArea?` true _array_element)
      (if (`self.IsReady?`)
        (`self.SequenceEvent`)))))

(event `SetReady`
  (set `self.IsReady?` true)
  (if (`self.IsBananaInArea?`)
    (`self.SequenceEvent`)))

(event `SequenceEvent`
  (bind _returnvalue (`GameplayStatics.GetPlayerCharacter` 0))
  ;[1 1 1] disable movement and mesh, play sequence, then reenable mesh and movement
  ;;[1 1 1] Destroy scene banana
  (bind _outactors (`GameplayStatics.GetAllActorsOfClass` "/Game/Blueprints/BP_Banana.BP_Banana_C"))
  (for _array_element _outactors
    (`self.K2_DestroyActor` _array_element))
  ;;[1 1 1] Kill bob in scene
  (bind _outactors_2 (`GameplayStatics.GetAllActorsOfClass` "/Game/Characters/Animations/Chad/BP_Bob.BP_Bob_C"))
  (for _array_element_2 _outactors_2
    (bind _asbp_bob (cast `/Game/Characters/Animations/Chad/BP_Bob` _array_element_2))
    (`self.K2_DestroyActor` _asbp_bob))
  (`ActorComponent.ToggleActive` (`Character.CharacterMovement` _returnvalue))
  (`SceneComponent.SetVisibility` (`Character.Mesh` _returnvalue) false true)
  (bind (_outactor _returnvalue_2) (`LevelSequencePlayer.CreateLevelSequencePlayer` (`self.LS`)))
  (`MovieSceneSequencePlayer.Play` (`LevelSequenceActor.SequencePlayer` _outactor))
  (add `MovieSceneSequencePlayer.OnFinished` _returnvalue_2 (delegate `Sequence finished`)))

(event `Sequence finished`
  (bind _returnvalue (`GameplayStatics.GetPlayerCharacter` 0))
  (bind _bobfallen (`self.BobFallen`))
  ;[1 1 1] disable movement and mesh, play sequence, then reenable mesh and movement
  (`ActorComponent.ToggleActive` (`Character.CharacterMovement` _returnvalue))
  (`SceneComponent.SetVisibility` (`Character.Mesh` _returnvalue) true true)
  (`SceneComponent.SetVisibility` _bobfallen true true)
  (`PrimitiveComponent.SetCollisionEnabled` _bobfallen "QueryAndPhysics")
  ;;[1 1 1] Set chandelier ready
  (bind _outactors (`GameplayStatics.GetAllActorsOfClass` "/Game/Blueprints/BP_Chandelier.BP_Chandelier_C"))
  (for _array_element _outactors
    (bind _asbp_chandelier (cast `/Game/Blueprints/BP_Chandelier` _array_element))
    (set `/Game/Blueprints/BP_Chandelier.IsReady` true _asbp_chandelier)
    ;;[1 1 1] Kill chad
    (bind _outactors_2 (`GameplayStatics.GetAllActorsOfClass` "/Game/Characters/Animations/Chad/BP_Chad.BP_Chad_C"))
    (for _array_element_2 _outactors_2
      (bind _asbp_chad (cast `/Game/Characters/Animations/Chad/BP_Chad` _array_element_2))
      (`self.K2_DestroyActor` _asbp_chad))))

(fn `UserConstructionScript`)