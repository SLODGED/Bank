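; Clickable keypad button actor that reports its value to an owning keypad actor.
; Hovering swaps the button mesh to a gold material and back to steel, with a ResetButtons event also restoring steel.
; Clicks call ButtonEntered on the keypad reference with the button's text plus confirm and backspace flags.
; The construction script writes the configured text onto the button's label.
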(event `self.Button.OnBeginCursorOver`
  (params (TouchedComponent :type "PrimitiveComponent Object Reference"))
  ;[1 1 1] Hovered and unhovered effects
  (`PrimitiveComponent.SetMaterial` (`self.Button`) 0 "/Game/StarterContent/Materials/M_Metal_Gold.M_Metal_Gold") ; Material to switch to when hovered
)

(event `self.Button.OnEndCursorOver`
  (params (TouchedComponent :type "PrimitiveComponent Object Reference"))
  ;[1 1 1] Hovered and unhovered effects
  (`PrimitiveComponent.SetMaterial` (`self.Button`) 0 "/Game/StarterContent/Materials/M_Metal_Steel.M_Metal_Steel" :!label _label))

(event `Reset Buttons`
  ;[1 1 1] Hovered and unhovered effects
  (goto _label))

(event `self.Button.OnClicked`
  (params (TouchedComponent :type "PrimitiveComponent Object Reference") (ButtonPressed :type "Key Structure"))
  ;[1 1 1] On button clicked event
  (`/Game/Blueprints/Keypad_System/Keypad_Actor.Button Entered` (`self.KeypadActorRef`) (`self.NoText`) (`self.ConfirmedButton?`) (`self.Backspace`)))

(fn `UserConstructionScript`
  ;[1 1 1] Setting text on button
  (`TextRenderComponent.K2_SetText` (`self.ButtonNo`) (`self.NoText`)))