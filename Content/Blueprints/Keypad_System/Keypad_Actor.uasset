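; Interactive passcode keypad actor that registers itself with the third-person character while the player overlaps its collision box.
; Interaction blends the view to the keypad camera, enables mouse clicking and hands itself to twelve child-actor buttons.
; Button events edit a dot-placeholder display, and confirm compares it to KeypadCode with text, glow and sound feedback.
; Both results reset buttons after a delay; success also restores the player view and destroys the collision box.
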(event `self.CollisionBox.OnComponentBeginOverlap`
  (params (OverlappedComponent :type "PrimitiveComponent Object Reference") (OtherActor :type "Actor Object Reference") (OtherComp :type "PrimitiveComponent Object Reference") (OtherBodyIndex :type Integer) (bFromSweep :type Boolean) (SweepResult :type "HitResult Structure (by ref)"))
  ;[1 1 1] On overlap events, set player references
  (if (== OtherActor (`GameplayStatics.GetPlayerPawn` 0))
    (bind _asbp_third_person_character (cast `/Game/ThirdPerson/Blueprints/BP_ThirdPersonCharacter` OtherActor))
    (set `/Game/ThirdPerson/Blueprints/BP_ThirdPersonCharacter.Keypad Interact Actor` self _asbp_third_person_character)
    (set `self.Player Ref` _asbp_third_person_character)))

(event `self.CollisionBox.OnComponentEndOverlap`
  (params (OverlappedComponent :type "PrimitiveComponent Object Reference") (OtherActor :type "Actor Object Reference") (OtherComp :type "PrimitiveComponent Object Reference") (OtherBodyIndex :type Integer))
  ;[1 1 1] On overlap events, set player references
  (if (== OtherActor (`GameplayStatics.GetPlayerPawn` 0))
    (bind _asbp_third_person_character (cast `/Game/ThirdPerson/Blueprints/BP_ThirdPersonCharacter` OtherActor))
    (set `/Game/ThirdPerson/Blueprints/BP_ThirdPersonCharacter.Keypad Interact Actor` null _asbp_third_person_character)
    (set `self.Player Ref` null)))

(event `On Interacted`
  (bind _returnvalue (`GameplayStatics.GetPlayerController` 0))
  (bind _enteredcodetext (`self.EnteredCodeText`))
  ;[1 1 1] On player interaction with keypad
  (`PlayerController.SetViewTargetWithBlend` (`GameplayStatics.GetPlayerController` 0) (`ActorComponent.GetOwner` (`self.Camera`)) 0.4 "VTBlend_Linear" 0.0 false)
  (bind _output_get (set `PlayerController.bShowMouseCursor` true _returnvalue :!label _label))
  (bind _output_get_2 (set `PlayerController.bEnableClickEvents` _output_get _returnvalue))
  (set `PlayerController.bEnableMouseOverEvents` _output_get_2 _returnvalue)
  (`TextRenderComponent.K2_SetText` _enteredcodetext (`KismetSystemLibrary.MakeLiteralText` (`KismetTextLibrary.Conv_StringToText` (`KismetStringLibrary.GetSubstring` "........." 0 (`KismetStringLibrary.Len` (`self.Keypad_Code`))))))
  (`TextRenderComponent.SetTextRenderColor` _enteredcodetext (make `Color` 1 1 1 255))
  (bind _output_get_3 (set `self.ButtonsArray` (`|MakeArray` (`self.Button1`) (`self.Button2`) (`self.Button3`) (`self.Button4`) (`self.Button5`) (`self.Button6`) (`self.Button7`) (`self.Button8`) (`self.Button9`) (`self.ButtonConfirm`) (`self.Button0`) (`self.Button_Back`))))
  (for _array_element _output_get_3
    (bind _askeypad_button_actor (cast `/Game/Blueprints/Keypad_System/KeypadButton_Actor` (`ChildActorComponent.ChildActor` _array_element)))
    (set `/Game/Blueprints/Keypad_System/KeypadButton_Actor.KeypadActorRef` self _askeypad_button_actor)))

(event `Initiate`
  ;[1 1 1] On player interaction with keypad
  (goto _label))

(event `Button Entered`
  (params (Value :type Text) (`Confirmed?` :type Boolean) (Backspace :type Boolean))
  (bind _enteredcodetext (`self.EnteredCodeText`))
  ;[1 1 1] Event confirmed when button is pressed
  (if `Confirmed?`
    (`self.On Confirmed`)
    (elif Backspace
      (`self.Backspace`)
      (elif (`self.Can Enter`)
        (`GameplayStatics.PlaySound2D` null 1.0 1.0 0.0 null null) ; On clicked sound effect
        (`TextRenderComponent.K2_SetText` _enteredcodetext (`KismetTextLibrary.Conv_StringToText` (`KismetStringLibrary.Replace` (`KismetTextLibrary.Conv_TextToString` (`TextRenderComponent.Text` (`self.EnteredCodeText`))) (`KismetStringLibrary.GetSubstring` "........." 0 (`KismetStringLibrary.Len` (`self.Keypad_Code`))))))
        (`TextRenderComponent.K2_SetText` _enteredcodetext (`KismetTextLibrary.Conv_StringToText` (`KismetStringLibrary.Concat_StrStr` (`KismetTextLibrary.Conv_TextToString` (`TextRenderComponent.Text` (`self.EnteredCodeText`))) (`KismetTextLibrary.Conv_TextToString` Value))))
        (`TextRenderComponent.SetTextRenderColor` (`self.EnteredCodeText`) (make `Color` 255 255 255 255))))))

(event `Backspace`
  (bind _enteredcodetext (`self.EnteredCodeText`))
  (bind _returnvalue (`KismetTextLibrary.Conv_TextToString` (`TextRenderComponent.Text` _enteredcodetext)))
  ;[1 1 1] For Backspace
  (`TextRenderComponent.K2_SetText` _enteredcodetext (`KismetTextLibrary.Conv_StringToText` (`KismetStringLibrary.GetSubstring` _returnvalue 0 (- (`KismetStringLibrary.Len` _returnvalue) 1)))))

(event `On Confirmed`
  (bind _returnvalue (`GameplayStatics.GetPlayerController` 0))
  (bind _returnvalue_2 (`GameplayStatics.GetPlayerController` 0))
  (bind _enteredcodetext (`self.EnteredCodeText`))
  (bind _enteredcodetext_2 (`self.EnteredCodeText`))
  (if (`KismetStringLibrary.EqualEqual_StrStr` (`self.Keypad_Code`) (`KismetTextLibrary.Conv_TextToString` (`TextRenderComponent.Text` (`self.EnteredCodeText`))))
    (`|ExecutionSequence`
      (:`then_0`
        (`TextRenderComponent.K2_SetText` _enteredcodetext_2 "Correct Passcode")
        (`TextRenderComponent.SetTextRenderColor` _enteredcodetext_2 (make `Color` 0 255 0 255)) ; Colour for when passcode is correct
        (`PrimitiveComponent.SetMaterial` (`self.Keypad`) 2 "/Game/Blueprints/Keypad_System/Materials/Green_Glow.Green_Glow")
        (`KismetSystemLibrary.RetriggerableDelay` 2.0)
        (bind _output_get (set `PlayerController.bShowMouseCursor` false _returnvalue_2))
        (bind _output_get_2 (set `PlayerController.bEnableMouseOverEvents` _output_get _returnvalue_2))
        (set `PlayerController.bEnableClickEvents` _output_get_2 _returnvalue_2)
        (for _array_element (`self.ButtonsArray`)
          (bind _askeypad_button_actor (cast `/Game/Blueprints/Keypad_System/KeypadButton_Actor` (`ChildActorComponent.ChildActor` _array_element)))
          (`/Game/Blueprints/Keypad_System/KeypadButton_Actor.Reset Buttons` _askeypad_button_actor))
        (`PlayerController.SetViewTargetWithBlend` (`GameplayStatics.GetPlayerController` 0) (`ActorComponent.GetOwner` (`/Game/ThirdPerson/Blueprints/BP_ThirdPersonCharacter.FollowCamera` (cast `/Game/ThirdPerson/Blueprints/BP_ThirdPersonCharacter` (`GameplayStatics.GetPlayerPawn` 0) :!pure true))) 0.4 "VTBlend_Linear" 0.0 false)
        (`TextRenderComponent.K2_SetText` (`self.EnteredCodeText`) "")
        (`WidgetBlueprintLibrary.SetInputMode_GameOnly` (`GameplayStatics.GetPlayerController` 0))
        (`ActorComponent.K2_DestroyComponent` (`self.CollisionBox`)))
      (:`then_1`
        (set `self.Can Enter` false)
        (`GameplayStatics.PlaySound2D` null 1.0 1.0 0.0 null null)))
    (else
      (`|ExecutionSequence`
        (:`then_0`
          (`TextRenderComponent.K2_SetText` _enteredcodetext "Wrong Passcode")
          (`TextRenderComponent.SetTextRenderColor` _enteredcodetext (make `Color` 255 0 0 255)) ; Colour for when passcode is incorrect
          (`PrimitiveComponent.SetMaterial` (`self.Keypad`) 2 "/Game/Blueprints/Keypad_System/Materials/Red_Glow.Red_Glow")
          (`KismetSystemLibrary.RetriggerableDelay` 2.0)
          (bind _output_get_3 (set `PlayerController.bEnableMouseOverEvents` false _returnvalue))
          (set `PlayerController.bEnableClickEvents` _output_get_3 _returnvalue)
          (for _array_element_2 (`self.ButtonsArray`)
            (bind _askeypad_button_actor_2 (cast `/Game/Blueprints/Keypad_System/KeypadButton_Actor` (`ChildActorComponent.ChildActor` _array_element_2)))
            (`/Game/Blueprints/Keypad_System/KeypadButton_Actor.Reset Buttons` _askeypad_button_actor_2)))
        (:`then_1`
          (set `self.Can Enter` false)
          (`GameplayStatics.PlaySound2D` null 1.0 1.0 0.0 null null))))))

(fn `UserConstructionScript`)