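; A thrown banana actor that the player can pick back up, shown whole or peeled according to the character's BananaPeeled flag.
; On spawn it simulates physics with pickup locked, then a fixed delay freezes it and enables pickup.
; Player overlap with its box then calls BananaPickup on the character and destroys the actor.
; A hit while IsBananaInArea freezes it and disables pickup, though a still-pending delay re-enables pickup.
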(event `self.ReceiveBeginPlay`
  ;[1 1 1] Banana Throw
  (set `self.CanPickup` false)
  ;;[1 1 1] Switch mesh depending
  (bind _asbp_third_person_character (cast `/Game/ThirdPerson/Blueprints/BP_ThirdPersonCharacter` (`GameplayStatics.GetPlayerCharacter` 0)))
  (if (`/Game/ThirdPerson/Blueprints/BP_ThirdPersonCharacter.BananaPeeled?` _asbp_third_person_character)
    (`StaticMeshComponent.SetStaticMesh` (`self.Banana`) "/Game/Meshes/BananaPeel/SM_BananaPeel.SM_BananaPeel")
    (else
      (`StaticMeshComponent.SetStaticMesh` (`self.Banana`) "/Game/Meshes/Banana/SM_Banana.SM_Banana")))
  ;;[1 1 1] Simulates until fallen
  (`PrimitiveComponent.SetSimulatePhysics` (`self.Banana`) true)
  (`KismetSystemLibrary.Delay` 5.0)
  (`PrimitiveComponent.SetSimulatePhysics` (`self.Banana`) false)
  (set `self.CanPickup` true))

(event `self.Box.OnComponentBeginOverlap`
  (params (OverlappedComponent :type "PrimitiveComponent Object Reference") (OtherActor :type "Actor Object Reference") (OtherComp :type "PrimitiveComponent Object Reference") (OtherBodyIndex :type Integer) (bFromSweep :type Boolean) (SweepResult :type "HitResult Structure (by ref)"))
  (bind _returnvalue (`GameplayStatics.GetPlayerCharacter` 0))
  ;[1 1 1] Banana Pickup
  (if (== OtherActor _returnvalue)
    (if (`self.CanPickup`)
      (bind _asbp_third_person_character (cast `/Game/ThirdPerson/Blueprints/BP_ThirdPersonCharacter` _returnvalue))
      (`/Game/ThirdPerson/Blueprints/BP_ThirdPersonCharacter.BananaPickup` _asbp_third_person_character)
      (`self.K2_DestroyActor`))))

(event `self.Banana.OnComponentHit`
  (params (HitComponent :type "PrimitiveComponent Object Reference") (OtherActor :type "Actor Object Reference") (OtherComp :type "PrimitiveComponent Object Reference") (NormalImpulse :type "Vector Structure") (Hit :type "HitResult Structure (by ref)"))
  ;[1 1 1] If in area, stop moving & disable pickiup
  (if (`self.IsBananaInArea?`)
    (set `self.CanPickup` false)
    (`PrimitiveComponent.SetSimulatePhysics` (`self.Banana`) false)))

(fn `UserConstructionScript`)