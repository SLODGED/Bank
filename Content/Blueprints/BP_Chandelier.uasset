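; BP_Chandelier is a chandelier actor whose trigger plays a level sequence when the player character overlaps it while IsReady is true.
; The overlap starts a newly created sequence player, toggles the character's movement component and hides its mesh along with attached children.
; A finish callback is bound but empty, so this Blueprint never restores movement or visibility, nor does it set IsReady.
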(event `self.Trigger.OnComponentBeginOverlap`
  (params (OverlappedComponent :type "PrimitiveComponent Object Reference") (OtherActor :type "Actor Object Reference") (OtherComp :type "PrimitiveComponent Object Reference") (OtherBodyIndex :type Integer) (bFromSweep :type Boolean) (SweepResult :type "HitResult Structure (by ref)"))
  (bind _returnvalue (`GameplayStatics.GetPlayerCharacter` 0))
  ;[1 1 1] if player collides & If Ready, play sequence
  (if (`self.IsReady`)
    (if (== OtherActor _returnvalue)
      (`self.Play Sequence`)
      (`ActorComponent.ToggleActive` (`Character.CharacterMovement` _returnvalue))
      (`SceneComponent.SetVisibility` (`Character.Mesh` _returnvalue) false true))))

(event `Play Sequence`
  ;[1 1 1] Play sequence & something if sequence finished
  (bind (_outactor _returnvalue) (`LevelSequencePlayer.CreateLevelSequencePlayer` (`self.LS`)))
  (`MovieSceneSequencePlayer.Play` (`LevelSequenceActor.SequencePlayer` _outactor))
  (add `MovieSceneSequencePlayer.OnFinished` _returnvalue (delegate `Sequence finished`)))

(event `Sequence finished`
  ;[1 1 1] Play sequence & something if sequence finished
)

(fn `UserConstructionScript`)