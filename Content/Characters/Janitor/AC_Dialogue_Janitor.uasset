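; Dialogue component for the Janitor NPC, overriding the Dialogue function with a tree branched on DialogueTreeIndex.
; The first tree has the player demand the uniform, where threatening him advances the index, closes the conversation and makes every NPC_Janitor move and idle.
; Backing out clears progress and idles the janitors.
; The second tree is a short brush-off line that ends the same way.
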(fn `Dialogue`
  (`parent.Dialogue`)
  (switch `int` (`self.DialogueTreeIndex`)
    (:`0`
      (bind (_state _optionindex) (`self.AddDialogue` "Janitor" "What do you want?" (`|MakeArray` "Hey old man, I’m gonna need your uniform." :!type "Text") null "/Game/Characters/Janitor/Animations/Talking.Talking"))
      (switch `/Game/Dialogue/Enum_DialogueState` _state
        (:`NewEnumerator0`
          (switch `int` _optionindex
            (:`0`
              (bind (_state_2 _optionindex_2) (`self.AddDialogue` "Janitor" "An what makes ye think I’m gunna give it to ye?" (`|MakeArray` "The bullet I’m gonna put between your eyes." "Sorry I forgot why I'm even talkin to ya." :!type "Text") "/Game/Dialogue/Audio/2.2" "/Game/Characters/Janitor/Animations/Talking.Talking"))
              (switch `/Game/Dialogue/Enum_DialogueState` _state_2
                (:`NewEnumerator0`
                  (switch `int` _optionindex_2
                    (:`0`
                      (bind (_state_3 _optionindex_3) (`self.AddDialogue` "Janitor" "Understandable. Here you go." (`|MakeArray` "And get out of my way" :!type "Text") null "/Game/Characters/Janitor/Animations/Talking.Talking"))
                      (switch `/Game/Dialogue/Enum_DialogueState` _state_3
                        (:`NewEnumerator0`
                          (switch `int` _optionindex_3
                            (:`0`
                              (bind _state_4 (`self.AddDialogue` "Janitor" "Fine" (`|MakeArray` "Thank you very much :)" :!type "Text") null "/Game/Characters/Janitor/Animations/Talking.Talking"))
                              (switch `/Game/Dialogue/Enum_DialogueState` _state_4
                                (:`NewEnumerator0`
                                  (`self.SetDialogueTreeIndex` 1)
                                  (`self.CloseConversation`)
                                  (bind _outactors (`GameplayStatics.GetAllActorsOfClass` "/Game/Characters/Janitor/NPC_Janitor.NPC_Janitor_C"))
                                  (for _array_element _outactors
                                    (bind _asnpc_janitor (cast `/Game/Characters/Janitor/NPC_Janitor` _array_element))
                                    (`/Game/Characters/Janitor/NPC_Janitor.Move` _asnpc_janitor)
                                    (`/Game/Characters/Janitor/NPC_Janitor.Idle` _asnpc_janitor)))))))))
                    (:`1`
                      (`self.ClearDialogueProgress`)
                      (`self.CloseConversation`)
                      (bind _outactors_2 (`GameplayStatics.GetAllActorsOfClass` "/Game/Characters/Janitor/NPC_Janitor.NPC_Janitor_C" :!label _label))
                      (for _array_element_2 _outactors_2
                        (bind _asnpc_janitor_2 (cast `/Game/Characters/Janitor/NPC_Janitor` _array_element_2))
                        (`/Game/Characters/Janitor/NPC_Janitor.Idle` _asnpc_janitor_2)))))))))))
    (:`1`
      (bind _state_5 (`self.AddDialogue` "Janitor" "The doors already open, leave me alone. I a cat at home" (`|MakeArray` "Fine, watch your step bucko" :!type "Text") null "/Game/Characters/Janitor/Animations/Talking.Talking"))
      (switch `/Game/Dialogue/Enum_DialogueState` _state_5
        (:`NewEnumerator0`
          (`self.ClearDialogueProgress`)
          (`self.CloseConversation`)
          (goto _label))))))