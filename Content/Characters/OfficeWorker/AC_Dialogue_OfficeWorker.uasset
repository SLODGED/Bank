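; Dialogue component for the office worker NPC, defining a short, grumpy conversation with the player.
; It overrides the parent Dialogue function and switches on DialogueTreeIndex, chaining AddDialogue calls with talking animation and response options.
; The first branch picks randomized lines and advances the index only if the player asks what the worker is doing.
; The follow-up branch delivers an annoyed brush-off, then clears dialogue progress and closes the conversation.
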(fn `Dialogue`
  (`parent.Dialogue`)
  (switch `int` (`self.DialogueTreeIndex`)
    (:`0`
      (bind (_state _optionindex) (`self.AddDialogue` "Worker" (select `int` (`KismetMathLibrary.RandomIntegerInRange` 0 4) :`0` "..." :`1` "I hate this job" :`2` "God, this place sucks" :`3` "*Cough Cough*" :`4` "..." :!type "Text") (`|MakeArray` "What are you doing?" "(Leave)" :!type "Text") null "/Game/Characters/Janitor/Animations/Talking.Talking"))
      (switch `/Game/Dialogue/Enum_DialogueState` _state
        (:`NewEnumerator0`
          (switch `int` _optionindex
            (:`0`
              (bind _state_2 (`self.AddDialogue` "Worker" (select `int` (`KismetMathLibrary.RandomIntegerInRange` 0 1) :`0` "Working, now please leave me alone" :`1` "Pretending to do work, just leave me be" :`2` "" :`3` "" :`4` "" :!type "Text") (`|MakeArray` "Fine" :!type "Text") null "/Game/Characters/Janitor/Animations/Talking.Talking"))
              (switch `/Game/Dialogue/Enum_DialogueState` _state_2
                (:`NewEnumerator0`
                  (`self.SetDialogueTreeIndex` 1)
                  (`self.CloseConversation`))))
            (:`1`
              (`self.SetDialogueTreeIndex` 0)
              (`self.CloseConversation`))))))
    (:`1`
      (bind _state_3 (`self.AddDialogue` "Worker" "I thought I told you to leave me alone" (`|MakeArray` "Whatever bud" "Fuck you" :!type "Text") null "/Game/Characters/Janitor/Animations/Talking.Talking"))
      (switch `/Game/Dialogue/Enum_DialogueState` _state_3
        (:`NewEnumerator0`
          (`self.ClearDialogueProgress`)
          (`self.CloseConversation`))))))